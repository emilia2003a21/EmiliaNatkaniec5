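; BP_FPS_01 is a basic first-person player Blueprint in the ModularBuildingSet folder, providing walk and look controls.
; Two movement axis inputs feed AddMovementInput along the capsule component's forward and right vectors.
; Two turning axis inputs pass straight to controller yaw and pitch input, and the construction script is empty.
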(event Input|AxisEvents|InputAxisMovementupdown
  (params (AxisValue :type Float%20%28single-precision%29))
  (Pawn|Input|AddMovementInput (Math|Vector|GetForwardVector (Variables|Collision|GetCapsuleComponent)) AxisValue false))

(event Input|AxisEvents|InputAxismovementRightLeft
  (params (AxisValue :type Float%20%28single-precision%29))
  (Pawn|Input|AddMovementInput (Math|Vector|GetRightVector (Variables|Collision|GetCapsuleComponent)) AxisValue false))

(event Input|AxisEvents|InputAxisturningX
  (params (AxisValue :type Float%20%28single-precision%29))
  (Pawn|Input|AddControllerYawInput AxisValue))

(event Input|AxisEvents|InputAxisturningY
  (params (AxisValue :type Float%20%28single-precision%29))
  (Pawn|Input|AddControllerPitchInput AxisValue))

(fn ConstructionScript)